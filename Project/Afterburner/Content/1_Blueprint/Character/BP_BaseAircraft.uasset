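; BP_BaseAircraft is a base aircraft Blueprint that handles player movement input through Enhanced Input.
; On BeginPlay it adds the IMC_BaseAircraft mapping context to its player controller's input subsystem.
; Forward and right move actions pass their values to MoveForwardInput and MoveRightInput, whose logic is outside this graph, and set movement flags.
; IsMoveForward clears on completion, while IsMoveRight is set true on both trigger and completion.
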(event `self.ReceiveBeginPlay`
  ;[1 1 1] BeginPlay
  (bind `_as플레이어_컨트롤러` (cast `PlayerController` (`self.GetController`)))
  (bind _returnvalue (pcsubsystem `EnhancedInputLocalPlayerSubsystem` `_as플레이어_컨트롤러`))
  (`/Engine/EditorBlueprintResources/StandardMacros.IsValid` _returnvalue
    (:`Is Valid`
      (message `EnhancedInputSubsystemInterface.AddMappingContext` _returnvalue "/Game/2_Input/Player/IMC_BaseAircraft.IMC_BaseAircraft" 0 (struct)))))

(event `EnhancedInput|/Game/2_Input/Player/InputAction/IA_MoveForward`
  (params (ActionValue :type "Float (double-precision)") (ElapsedSeconds :type "Float (double-precision)") (TriggeredSeconds :type "Float (double-precision)") (InputAction :type "InputAction Object Reference" :default "/Game/2_Input/Player/InputAction/IA_MoveForward.IA_MoveForward"))
  ;[1 1 1] Move
  (:`Triggered`
    (`self.MoveForwardInput` ActionValue)
    (set `self.bIsMoveForward` true))
  (:`Completed`
    (set `self.bIsMoveForward` false)))

(event `EnhancedInput|/Game/2_Input/Player/InputAction/IA_MoveRight`
  (params (ActionValue :type "Float (double-precision)") (ElapsedSeconds :type "Float (double-precision)") (TriggeredSeconds :type "Float (double-precision)") (InputAction :type "InputAction Object Reference" :default "/Game/2_Input/Player/InputAction/IA_MoveRight.IA_MoveRight"))
  ;[1 1 1] Move
  (:`Triggered`
    (`self.MoveRightInput` ActionValue)
    (set `self.bIsMoveRight` true))
  (:`Completed`
    (set `self.bIsMoveRight` true)))

(fn `UserConstructionScript`)